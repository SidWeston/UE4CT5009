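; BP_Lift is a lift actor that moves while the player character stands in its trigger and returns when they leave.
; BeginPlay stores the start location and converts LiftEndPosition from an offset into an end point relative to it.
; LiftTrigger overlaps from DualViewCharacterControllerBP play or reverse LiftTimeline, whose track lerps the actor between both points without sweeping.
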(event `self.ReceiveBeginPlay`
  (bind _returnvalue (`self.K2_GetActorLocation`))
  (set `self.LiftStartPosition` _returnvalue)
  (set `self.LiftEndPosition` (+ (`self.LiftEndPosition`) _returnvalue)))

(event `self.LiftTrigger.OnComponentBeginOverlap`
  (params (OverlappedComponent :type "PrimitiveComponent Object Reference") (OtherActor :type "Actor Object Reference") (OtherComp :type "PrimitiveComponent Object Reference") (OtherBodyIndex :type Integer) (bFromSweep :type Boolean) (SweepResult :type "HitResult Structure (by ref)"))
  (cast `/Game/Blueprints/CharacterControllers/DualViewCharacterControllerBP` OtherActor)
  (bind (_direction _newtrack_0) (`Timeline|LiftTimeline` :!label _label)
    (:`Update`
      (`self.K2_SetActorRelativeLocation` (`KismetMathLibrary.VLerp` (`self.LiftStartPosition`) (`self.LiftEndPosition`) _newtrack_0)))))

(event `self.LiftTrigger.OnComponentEndOverlap`
  (params (OverlappedComponent :type "PrimitiveComponent Object Reference") (OtherActor :type "Actor Object Reference") (OtherComp :type "PrimitiveComponent Object Reference") (OtherBodyIndex :type Integer))
  (cast `/Game/Blueprints/CharacterControllers/DualViewCharacterControllerBP` OtherActor)
  (goto _label :!via `Reverse`))

(fn `UserConstructionScript`)