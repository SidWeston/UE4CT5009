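; Swinging door that opens automatically for a ThirdPersonCharacter, in a direction set by which side it enters from.
; Front and back trigger boxes drive separate timelines that lerp the mesh's relative rotation from the actor's rotation toward TargetRotation or its negation.
; Both timelines toggle a shared CanOpen flag on finishing, so leaving a box reverses its timeline only while the flag is false.
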(event `self.FrontBox.OnComponentBeginOverlap`
  (params (OverlappedComponent :type "PrimitiveComponent Object Reference") (OtherActor :type "Actor Object Reference") (OtherComp :type "PrimitiveComponent Object Reference") (OtherBodyIndex :type Integer) (bFromSweep :type Boolean) (SweepResult :type "HitResult Structure (by ref)"))
  (cast `/Game/ThirdPersonBP/Blueprints/ThirdPersonCharacter` OtherActor)
  (if (`self.CanOpen`)
    (bind (_direction _door) (`Timeline|DoorOpen` :!label _label)
      (:`Update`
        (`SceneComponent.K2_SetRelativeRotation` (`self.DoorMesh`) (`KismetMathLibrary.RLerp` (`self.K2_GetActorRotation`) (`self.TargetRotation`) _door) false false))
      (:`Finished`
        (if (`self.CanOpen`)
          (set `self.CanOpen` false)
          (else
            (set `self.CanOpen` true)))))))

(event `self.FrontBox.OnComponentEndOverlap`
  (params (OverlappedComponent :type "PrimitiveComponent Object Reference") (OtherActor :type "Actor Object Reference") (OtherComp :type "PrimitiveComponent Object Reference") (OtherBodyIndex :type Integer))
  (cast `/Game/ThirdPersonBP/Blueprints/ThirdPersonCharacter` OtherActor)
  (if (not (`self.CanOpen`))
    (goto _label :!via `Reverse`)))

(event `self.BackBox.OnComponentBeginOverlap`
  (params (OverlappedComponent :type "PrimitiveComponent Object Reference") (OtherActor :type "Actor Object Reference") (OtherComp :type "PrimitiveComponent Object Reference") (OtherBodyIndex :type Integer) (bFromSweep :type Boolean) (SweepResult :type "HitResult Structure (by ref)"))
  (bind (_targetrotation_roll _targetrotation_pitch _targetrotation_yaw) (`KismetMathLibrary.BreakRotator` (`self.TargetRotation`)))
  (cast `/Game/ThirdPersonBP/Blueprints/ThirdPersonCharacter` OtherActor)
  (if (`self.CanOpen`)
    (bind (_direction _door) (`Timeline|DoorReverseOpen` :!label _label_2)
      (:`Update`
        (`SceneComponent.K2_SetRelativeRotation` (`self.DoorMesh`) (`KismetMathLibrary.RLerp` (`self.K2_GetActorRotation`) (`KismetMathLibrary.MakeRotator` (* _targetrotation_roll -1.0) (* _targetrotation_pitch -1.0) (* _targetrotation_yaw -1.0)) _door) false false))
      (:`Finished`
        (if (`self.CanOpen`)
          (set `self.CanOpen` false)
          (else
            (set `self.CanOpen` true)))))))

(event `self.BackBox.OnComponentEndOverlap`
  (params (OverlappedComponent :type "PrimitiveComponent Object Reference") (OtherActor :type "Actor Object Reference") (OtherComp :type "PrimitiveComponent Object Reference") (OtherBodyIndex :type Integer))
  (cast `/Game/ThirdPersonBP/Blueprints/ThirdPersonCharacter` OtherActor)
  (if (not (`self.CanOpen`))
    (goto _label_2 :!via `Reverse`)))

(fn `UserConstructionScript`)